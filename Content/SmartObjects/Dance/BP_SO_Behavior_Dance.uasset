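; Smart object behavior for dancing that toggles motive regeneration on the Sim that triggers it.
; It takes the motive from the first activity tag of the owner's cached smart object definition, then finds the BP_Motives component on the BP_Sim avatar.
; It switches regen on for that motive, calls the parent trigger logic, then switches regen off directly after that call.
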(event EventOnTriggeredCharacter
  (params (Avatar :type Character%20Object%20Reference) (Config :type Gameplay%20Behavior%20Config%20Object%20Reference) (SmartObjectOwner :type Actor%20Object%20Reference))
  (Variables|Default|SetAvatar Avatar)
  (Variables|Default|SetConfig Config)
  (Variables|Default|SetSmart%20Object%20Owner SmartObjectOwner)
  (Variables|Default|SetMotive (Utilities|Array|Get(acopy) (.gameplaytags (Class|SmartObjectDefinition|GetActivityTags (Variables|/Script/SmartObjectsModule.SmartObjectComponent|GetCachedDefinitionAssetVariation (Actor|GetComponentbyClass (Variables|Default|GetSmart%20Object%20Owner) "/Script/SmartObjectsModule.SmartObjectComponent"))))))
  (bind _asbp_sim (Utilities|Casting|CastToBP_Sim (Variables|Default|GetAvatar)))
  (bind _output_get (Variables|Default|SetMotives (Actor|GetComponentbyClass _asbp_sim "/Game/Characters/BP_Motives.BP_Motives_C")))
  (Class|Motives|SetRegenState _output_get (Variables|Default|GetMotive) true)
  (|CallParentFunction (Variables|Default|GetAvatar) (Variables|Default|GetConfig) (Variables|Default|GetSmart%20Object%20Owner))
  (Class|Motives|SetRegenState (Variables|Default|GetMotives) (Variables|Default|GetMotive) false))