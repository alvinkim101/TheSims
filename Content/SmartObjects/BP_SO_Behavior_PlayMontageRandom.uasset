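; Smart Object behavior that has a Sim play a random montage at the object while it regenerates a motive.
; On trigger it casts the avatar to BP_Sim and takes the motive from the first activity tag of the Smart Object definition.
; Regen for that motive is switched on while the montage plays and off when it completes or is interrupted.
; An empty montage list logs a warning and ends the behavior.
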(event GameplayBehavior|EventOnTriggeredCharacter
  (params (Avatar :type Character%20Object%20Reference) (Config :type Gameplay%20Behavior%20Config%20Object%20Reference) (SmartObjectOwner :type Actor%20Object%20Reference))
  (bind _asbp_sim (Utilities|Casting|CastToBP_Sim Avatar)
    (:then
      (bind _output_get (Variables|Default|SetAvatar _asbp_sim))
      (Variables|Default|SetMotives (Variables|/Game/Characters/BP_Sim.BP_Sim_C|GetBP_Motives _output_get))
      (bind _output_get_2 (Variables|Default|SetSmart%20Object%20Owner SmartObjectOwner))
      (Variables|Default|SetMotive (Utilities|Array|Get(acopy) (.gameplaytags (Class|SmartObjectDefinition|GetActivityTags (Variables|/Script/SmartObjectsModule.SmartObjectComponent|GetCachedDefinitionAssetVariation (Actor|GetComponentbyClass _output_get_2 "/Script/SmartObjectsModule.SmartObjectComponent"))))))
      (if (Utilities|Array|IsNotEmpty (Variables|Default|GetMontage))
        (Class|Motives|SetRegenState (Variables|Default|GetMotives) (Variables|Default|GetMotive) true)
        (Animation|Montage|PlayMontage (Actor|GetComponentbyClass (Variables|Default|GetAvatar) "/Script/Engine.SkeletalMeshComponent") (.OutItem (Utilities|Array|Random (Variables|Default|GetMontage)))
          (:OnCompleted
            _)
          (:OnInterrupted
            _))
        (Class|Motives|SetRegenState (Variables|Default|GetMotives) (Variables|Default|GetMotive) false)
        (else
          (Development|PrintString 0 (Utilities|String|Append (Utilities|GetDisplayName (Variables|Default|GetSmart%20Object%20Owner)) ": Montage not valid"))))
      (GameplayBehavior|EndBehavior (Variables|Default|GetAvatar)))
    (:CastFailed
      (GameplayBehavior|EndBehavior Avatar))))