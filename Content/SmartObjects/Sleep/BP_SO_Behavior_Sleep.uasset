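; Smart Object behavior that makes a Sim sleep on an object until its Energy motive is full.
; It snaps the Sim to the Smart Object component's transform, then plays a start montage.
; Regen of the motive named by the object's first activity tag turns on while random loop montages repeat until Energy is full.
; An end montage then plays, after which regen turns off and the behavior ends.
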(event GameplayBehavior|EventOnTriggeredCharacter
  (params (Avatar :type Character%20Object%20Reference) (Config :type Gameplay%20Behavior%20Config%20Object%20Reference) (SmartObjectOwner :type Actor%20Object%20Reference))
  (Variables|Default|SetSmart%20Object%20Owner SmartObjectOwner)
  (bind _asbp_sim (Utilities|Casting|CastToBP_Sim Avatar))
  (Variables|Default|SetSim _asbp_sim)
  (Variables|Default|SetMotives (Actor|GetComponentbyClass (Variables|Default|GetSim) "/Game/Characters/BP_Motives.BP_Motives_C"))
  (Variables|Default|SetMotive (Utilities|Array|Get(acopy) (.gameplaytags (Class|SmartObjectDefinition|GetActivityTags (Variables|/Script/SmartObjectsModule.SmartObjectComponent|GetCachedDefinitionAssetVariation (Actor|GetComponentbyClass (Variables|Default|GetSmart%20Object%20Owner) "/Script/SmartObjectsModule.SmartObjectComponent"))))))
  (Variables|Default|SetSkeletal%20Mesh (Actor|GetComponentbyClass (Variables|Default|GetSim) "/Script/Engine.SkeletalMeshComponent"))
  (Transformation|SetActorTransform (Variables|Default|GetSim) (Transformation|GetWorldTransform (Actor|GetComponentbyClass (Variables|Default|GetSmart%20Object%20Owner) "/Script/SmartObjectsModule.SmartObjectComponent")))
  (Animation|Montage|PlayMontage (Variables|Default|GetSkeletal%20Mesh) "/Game/Animations/AM_SleepStart.AM_SleepStart"
    (:OnBlendOut
      (Class|Motives|SetRegenState (Variables|Default|GetMotives) (Variables|Default|GetMotive) true)
      (if (not (Class|Motives|IsFull (Variables|Default|GetMotives) "(TagName=\"Motive.Energy\")")) :!label _label
        (Animation|Montage|PlayMontage (Variables|Default|GetSkeletal%20Mesh) (.OutItem (Utilities|Array|Random (Variables|Default|GetLoop)))
          (:OnBlendOut
            (goto _label)))
        (else
          (Animation|Montage|PlayMontage (Variables|Default|GetSkeletal%20Mesh) "/Game/Animations/AM_SleepEnd.AM_SleepEnd"
            (:OnCompleted
              (Class|Motives|SetRegenState (Variables|Default|GetMotives) (Variables|Default|GetMotive) false)
              (GameplayBehavior|EndBehavior (Variables|Default|GetSim)))))))))