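; BP_Sim is the AI-driven Sim character, which owns its own HUD widget.
; When an AI controller possesses it, it runs the BT_Sim behavior tree and creates a WBP_HUD bound to itself.
; ShowHUD and HideHUD add that stored widget to the viewport or remove it.
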(event EventBeginPlay)

(event Collision|EventActorBeginOverlap
  (params (OtherActor :type Actor%20Object%20Reference)))

(event EventTick
  (params (DeltaSeconds :type Float%20%28single-precision%29)))

(event EventPossessed
  (params (NewController :type Controller%20Object%20Reference))
  (bind _asaicontroller (Utilities|Casting|CastToAIController NewController))
  (AI|RunBehaviorTree _asaicontroller "/Game/AI/BT_Sim.BT_Sim")
  (CallFunction|CreateHUD))

(fn ConstructionScript)

(fn CreateHUD
  (bind _returnvalue (UserInterface|CreateWidget "/Game/UI/WBP_HUD.WBP_HUD_C" 0 self))
  (Variables|Default|SetHUD _returnvalue))

(fn ShowHUD
  (UserInterface|Viewport|AddtoViewport (Variables|Default|GetHUD) 0))

(fn HideHUD
  (Widget|RemovefromParent (Variables|Default|GetHUD)))