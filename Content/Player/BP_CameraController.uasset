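; Player controller for a Sim-style game that drives an edge-scrolling, zoomable camera and mouse selection of Sims.
; BeginPlay adds the Enhanced Input mapping context and shows the cursor.
; Tick moves the pawn's arrow component when the cursor nears a viewport edge, while zoom input slides the spring arm along its forward vector.
; Clicks trace under the cursor, selecting a BP_Sim and showing its HUD if none is selected, or deselecting on a miss.
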(event Input|EnhancedActionEvents|EnhancedInputActionIA_ClickSim
  (params (ActionValue :type Boolean) (ElapsedSeconds :type Float%20%28double-precision%29) (TriggeredSeconds :type Float%20%28double-precision%29) (InputAction :type Input%20Action%20Object%20Reference :default "/Game/Player/Input/IA_ClickSim.IA_ClickSim"))
  (bind (_hit _sim) (CallFunction|GetSimUnderCursor))
  (if _hit
    (if (not (Utilities|IsValid (Variables|Default|GetSelectedSim)))
      (bind _output_get (Variables|Default|SetSelectedSim _sim))
      (Default|ShowHUD _output_get))
    (elif (Utilities|IsValid (Variables|Default|GetSelectedSim))
      (Default|HideHUD (Variables|Default|GetSelectedSim))
      (Variables|Default|SetSelectedSim 0))))

(event Input|EnhancedActionEvents|EnhancedInputActionIA_CameraZoom
  (params (ActionValue :type Float%20%28double-precision%29) (ElapsedSeconds :type Float%20%28double-precision%29) (TriggeredSeconds :type Float%20%28double-precision%29) (InputAction :type Input%20Action%20Object%20Reference :default "/Game/Player/Input/IA_CameraZoom.IA_CameraZoom"))
  (CallFunction|ZoomCamera ActionValue))

(event EventTick
  (params (DeltaSeconds :type Float%20%28single-precision%29))
  (bind _returnvalue (Class|WidgetLayoutLibrary|GetMousePositiononViewport))
  (CallFunction|MoveCamera (/ (* _returnvalue (Class|WidgetLayoutLibrary|GetViewportScale)) (Viewport|GetViewportSize)) DeltaSeconds))

(event EventBeginPlay
  (bind _returnvalue (PlayerController|LocalPlayerSubsystems|GetEnhancedInputLocalPlayerSubsystem))
  (Utilities|IsValid _returnvalue
    (:Is%20Valid
      (Input|AddMappingContext _returnvalue "/Game/Player/Input/IMC_Player.IMC_Player" 0 "(bIgnoreAllPressedKeysUntilRelease=True,bForceImmediately=False,bNotifyUserSettings=False)")
      (Variables|Default|SetbShowMouseCursor true))))

(fn ConstructionScript)

(fn GetSimUnderCursor
  (bind _object (LocalVariables|GetObject))
  (bind _hitresult (Class|PlayerController|GetHitResultUnderCursorforObjects _object true))
  (bind (_bblockinghit _binitialoverlap _time _distance _location _impactpoint _normal _impactnormal _physmat _hitactor) (Collision|BreakHitResult _hitresult))
  (if _bblockinghit
    (bind _asbp_sim (Utilities|Casting|CastToBP_Sim _hitactor)
      (:then
        (return true _asbp_sim))
      (:CastFailed
        _)))
  (return false 0))

(fn MoveCamera
  (params (Position :type Vector%202D%20Structure%20%28by%20ref%29) (Delta%20Seconds :type Float%20%28double-precision%29%20%28by%20ref%29))
  (bind _returnvalue (Pawn|GetControlledPawn))
  (bind _returnvalue_2 (Actor|GetComponentbyClass _returnvalue "/Script/Engine.ArrowComponent"))
  (LocalVariables|SetX (.x Position))
  (LocalVariables|SetY (.y Position))
  (LocalVariables|SetDeltaSeconds Delta%20Seconds)
  (if (Utilities|IsValid _returnvalue_2)
    (LocalVariables|SetArrow _returnvalue_2)
    (if (<= (LocalVariables|GetX) 0.1)
      (bind _output_get (LocalVariables|SetNewX (Variables|Default|GetCameraMoveDelta)))
      (Math|Float|NegateFloat _output_get
        (:%20%20
          _))
      (elif (>= (LocalVariables|GetX) 0.9)
        (LocalVariables|SetNewX (Variables|Default|GetCameraMoveDelta))))
    (if (<= (LocalVariables|GetY) 0.1)
      (LocalVariables|SetNewY (Variables|Default|GetCameraMoveDelta))
      (elif (>= (LocalVariables|GetY) 0.9)
        (bind _output_get_2 (LocalVariables|SetNewY (Variables|Default|GetCameraMoveDelta)))
        (Math|Float|NegateFloat _output_get_2
          (:%20%20
            _))))
    (Transformation|AddRelativeLocation (LocalVariables|GetArrow) (Math|Vector|MakeVector (* (LocalVariables|GetNewY) (LocalVariables|GetDeltaSeconds)) (* (LocalVariables|GetNewX) (LocalVariables|GetDeltaSeconds)) 0.0) false false)))

(fn ZoomCamera
  (params (Action%20Value :type Float%20%28double-precision%29%20%28by%20ref%29))
  (bind _returnvalue (Pawn|GetControlledPawn))
  (bind _returnvalue_2 (Actor|GetComponentbyClass _returnvalue "/Script/Engine.SpringArmComponent"))
  (if (Utilities|IsValid _returnvalue_2)
    (Transformation|AddRelativeLocation _returnvalue_2 (* (* Action%20Value (Variables|Default|GetCameraZoomDelta)) (Math|Vector|GetForwardVector _returnvalue_2)) false false)))